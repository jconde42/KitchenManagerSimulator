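; BP_Door is a sliding door actor that opens for the player pawn, with Blue and Red types requiring a matching item and Gray needing none.
; Box overlap checks DoorType against the pawn's Items, then plays a shared timeline that moves the Door along relative Z, scaled by Displacement.
; Any end overlap on the Box reverses the timeline to close the door, without checking the actor or its items.
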(event `self.Box.OnComponentBeginOverlap`
  (params (OverlappedComponent :type "PrimitiveComponent Object Reference") (OtherActor :type "Actor Object Reference") (OtherComp :type "PrimitiveComponent Object Reference") (OtherBodyIndex :type Integer) (bFromSweep :type Boolean) (SweepResult :type "HitResult Structure (by ref)"))
  (bind _asbp_player_pawn (cast `/Game/Blueprints/Pawns/BP_PlayerPawn` OtherActor))
  (switch `/Game/Blueprints/Enums/EDoorType` (`self.DoorType`)
    (:`NewEnumerator0`
      (bind _items (`/Game/Blueprints/Pawns/BP_PlayerPawn.Items` _asbp_player_pawn))
      (if (`BlueprintSetLibrary.Set_Contains` _items (make `/Game/Blueprints/Structs/Items` "NewEnumerator1"))
        (bind (_direction _newtrack_0) (`Timeline|Timeline_0` :!label _label)
          (:`Update`
            (`SceneComponent.K2_SetRelativeLocation` (`self.Door`) (`KismetMathLibrary.MakeVector` 0.0 0.0 (* _newtrack_0 (`self.Displacement`))) false false)))))
    (:`NewEnumerator1`
      (if (`BlueprintSetLibrary.Set_Contains` _items (make `/Game/Blueprints/Structs/Items` "NewEnumerator0"))
        (goto _label)))
    (:`NewEnumerator2`
      (goto _label))))

(event `self.Box.OnComponentEndOverlap`
  (params (OverlappedComponent :type "PrimitiveComponent Object Reference") (OtherActor :type "Actor Object Reference") (OtherComp :type "PrimitiveComponent Object Reference") (OtherBodyIndex :type Integer))
  (goto _label :!via `Reverse`))

(fn `UserConstructionScript`)