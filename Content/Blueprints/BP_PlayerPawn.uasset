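; Player pawn that moves in its local XY plane from the MoveUp and MoveLeft axis inputs.
; Axis events cache their values, and Tick passes delta time to MoveXY, which maps up to X and left to Y.
; The vector's length is capped so diagonals are no faster, then scaled by MoveSpeed and delta time and applied as a swept local offset.
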(event `self.ReceiveTick`
  (params (DeltaSeconds :type "Float (single-precision)"))
  (`|ExecutionSequence`
    (:`then_0`
      (`self.MoveXY` DeltaSeconds))))

(event `InputAxis|MoveLeft`
  (params (AxisValue :type "Float (single-precision)"))
  ;[1 1 1] MoveLeft
  (set `self.MoveLeftValue` AxisValue))

(event `InputAxis|MoveUp`
  (params (AxisValue :type "Float (single-precision)"))
  ;[1 1 1] MoveUp
  (set `self.MoveUpValue` AxisValue))

(fn `MoveXY`
  (params (`Delta Seconds` :type "Float (double-precision)"))
  (`self.K2_AddActorLocalOffset` (* (`KismetMathLibrary.ClampVectorSize` (`KismetMathLibrary.MakeVector` (`self.MoveUpValue`) (`self.MoveLeftValue`)) -1.0 1.0) (* `Delta Seconds` (`self.MoveSpeed`))) true))

(fn `UserConstructionScript`)